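; BP_Marine is a player-controlled marine pawn with twin-stick style movement and aiming.
; MoveForward and MoveLeft axis inputs add movement along fixed world X and Y axes, independent of facing.
; Each Tick, UpdatePlayerAim converts the aim thumbstick axes to a yaw with atan2 and sets player controller 0's control rotation.
; Aim only updates while the stick's vector length exceeds the deadzone, so the last direction holds otherwise.
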(event EventBeginPlay)

(event Collision|EventActorBeginOverlap
  (params (OtherActor :type Actor%20Object%20Reference)))

(event EventTick
  (params (DeltaSeconds :type Float%20%28single-precision%29))
  (CallFunction|UpdatePlayerAim))

(event Input|AxisEvents|InputAxisMoveForward
  (params (AxisValue :type Float%20%28single-precision%29))
  (Pawn|Input|AddMovementInput "1.000000, 0, 0" AxisValue false))

(event Input|AxisEvents|InputAxisMoveLeft
  (params (AxisValue :type Float%20%28single-precision%29))
  (Pawn|Input|AddMovementInput "0.000000,1.000000, 0" AxisValue false))

(fn ConstructionScript)

(fn UpdatePlayerAim
  (if (CallFunction|IsThumbStickAboveDeadzone)
    (Pawn|SetControlRotation (Game|GetPlayerController 0) (Math|Rotator|MakeRotator 0.0 0.0 (Class|KismetMathLibrary|DegAtan2 (Input|AxisValues|GetThumStickAimRight) (Input|AxisValues|GetThumStickAimUp))))))

(fn IsThumbStickAboveDeadzone
  (return (> (Math|Vector2D|Vector2DLength (Math|Vector2D|MakeVector2D (Input|AxisValues|GetThumStickAimUp) (Input|AxisValues|GetThumStickAimRight))) (Variables|Default|GetThumStick%20DeadZone))))